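; Timer screen actor that writes the current date and time to a TextRender when the player enters its trigger sphere.
; A DoOnce gates the sphere's begin overlap before the Player tag and overlap checks, so the first overlap by any actor uses it up.
; End overlap only checks the tag, and the DoOnce reset and Timer_bp widget creation are disconnected and never run.
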(event OnComponentBeginOverlap(Sphere)
  (params (OverlappedComponent :type Primitive%20Component%20Object%20Reference) (OtherActor :type Actor%20Object%20Reference) (OtherComp :type Primitive%20Component%20Object%20Reference) (OtherBodyIndex :type Integer) (bFromSweep :type Boolean) (SweepResult :type Hit%20Result%20Structure%20%28by%20ref%29))
  (Utilities|FlowControl|DoOnce false
    (:Completed
      (if (Actor|ActorHasTag OtherActor "Player")
        (if (Collision|IsOverlappingActor (Variables|Default|GetSphere) (Game|GetPlayerCharacter 0) :!class /Script/Engine.PrimitiveComponent)
          (Rendering|Components|TextRender|SetText (Variables|Default|GetTextRender) (Class|KismetTextLibrary|AsTimeDateTime (Math|DateTime|Now))))))))

(event OnComponentEndOverlap(Sphere)
  (params (OverlappedComponent :type Primitive%20Component%20Object%20Reference) (OtherActor :type Actor%20Object%20Reference) (OtherComp :type Primitive%20Component%20Object%20Reference) (OtherBodyIndex :type Integer))
  (if (Actor|ActorHasTag OtherActor "Player")
    _))

(fn ConstructionScript)